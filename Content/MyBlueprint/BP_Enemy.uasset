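; BP_Enemy is an enemy actor that moves in a straight line at a constant speed.
; On BeginPlay it picks its direction once: a 30% chance to head toward the player pawn's position at that moment, otherwise its own forward vector.
; Each Tick, the Translate function moves it along that fixed direction, scaled by speed and delta time, without sweeping for collisions.
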(event `self.ReceiveBeginPlay`
  (if (< (`KismetMathLibrary.RandomIntegerInRange` 0 9) 3)
    ;[1 1 1] 30%
    (set `self.FirstForward` (`KismetMathLibrary.Normal` (- (`self.K2_GetActorLocation` (`GameplayStatics.GetPlayerPawn` 0)) (`self.K2_GetActorLocation`))))
    (else
      ;[1 1 1] 70% 확률
      (set `self.FirstForward` (`self.GetActorForwardVector`)))))

(event `self.ReceiveTick`
  (params (DeltaSeconds :type "Float (single-precision)"))
  (`self.Translate` (`self.Speed`) (`self.FirstForward`)))

(fn `Translate`
  (params (speed :type "Float (double-precision)") (direction :type "Vector Structure") (IsSweep :type Boolean))
  (`self.K2_SetActorLocation` (+ (* speed (`GameplayStatics.GetWorldDeltaSeconds`) (`KismetMathLibrary.Normal` direction)) (`self.K2_GetActorLocation`)) IsSweep))

(fn `UserConstructionScript`)