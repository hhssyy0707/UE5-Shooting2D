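; BP_Tail is an actor that continuously moves toward a target, which defaults to the player.
; On BeginPlay it looks up a BP_Player actor if Target is not already valid.
; Each Tick it steps along the normalized direction to Target at Speed, scaled by delta time, without sweeping for collision or stopping at a distance.
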(event `self.ReceiveBeginPlay`
  (`/Engine/EditorBlueprintResources/StandardMacros.IsValid` (`self.Target`)
    (:`Is Not Valid`
      (bind _returnvalue (`GameplayStatics.GetActorOfClass` "/Game/MyBlueprint/BP_Player.BP_Player_C"))
      (set `self.Target` _returnvalue))))

(event `self.ReceiveTick`
  (params (DeltaSeconds :type "Float (single-precision)"))
  (`self.K2_SetActorLocation` (+ (`self.K2_GetActorLocation`) (* DeltaSeconds (`self.Speed`) (`KismetMathLibrary.Normal` (- (`self.K2_GetActorLocation` (`self.Target`)) (`self.K2_GetActorLocation`)))))))

(fn `UserConstructionScript`)