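; BP_EnemyManager is an enemy spawner that periodically creates BP_Enemy actors at its Arrow component's transform.
; BeginPlay starts a looping timer by function name at the RespawnTime interval and stores its handle.
; Each spawn call first checks that the player pawn is valid, clearing the timer when it is not.
; Disconnected alternatives using an event timer and Tick accumulation remain in the graph but never run.
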(event `self.ReceiveBeginPlay`
  ;[1 1 1] 방법1
  ;[1 1 1] 방법2
  (bind _returnvalue (`KismetSystemLibrary.K2_SetTimer` null "Spawn Enemy" (`self.RespawnTime`) true 0.5))
  ;[1 1 1] 예외처리 (player 없어지면 에러남)
  (set `self.TimerHandleSpawnEnemy` _returnvalue))

(event `Custom Event BeginPlay`
  ;[1 1 1] 방법2
)

(event `SpawnEnemy`
  ;[1 1 1] 방법1
  (`self.Spawn Enemy`))

(event `self.ReceiveTick`
  (params (DeltaSeconds :type "Float (single-precision)")))

(fn `Spawn Enemy`
  (`/Engine/EditorBlueprintResources/StandardMacros.IsValid` (`GameplayStatics.GetPlayerPawn` 0)
    (:`Is Valid`
      (`|SpawnActorFromClass` "/Game/MyBlueprint/BP_Enemy.BP_Enemy_C" (`SceneComponent.K2_GetComponentToWorld` (`self.Arrow`)) "Undefined" "MultiplyWithRoot" null null))
    (:`Is Not Valid`
      (`KismetSystemLibrary.K2_ClearAndInvalidateTimerHandle` (`self.TimerHandleSpawnEnemy`)))))

(fn `UserConstructionScript`)