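; BP_Bullet is a projectile that flies straight along its forward vector and destroys enemies it overlaps.
; Each Tick calls a Translate function that moves the actor by Speed scaled by delta time, without sweeping.
; Overlapping a BP_Enemy spawns an explosion emitter at the enemy's location, then destroys both the enemy and the bullet.
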(event `self.ReceiveActorBeginOverlap`
  (params (OtherActor :type "Actor Object Reference"))
  (bind _asbp_enemy (cast `/Game/MyBlueprint/BP_Enemy` OtherActor))
  (`GameplayStatics.SpawnEmitterAtLocation` "/Game/StarterContent/Particles/P_Explosion.P_Explosion" (`self.K2_GetActorLocation` _asbp_enemy))
  (`self.K2_DestroyActor` _asbp_enemy)
  (`self.K2_DestroyActor`))

(event `self.ReceiveTick`
  (params (DeltaSeconds :type "Float (single-precision)"))
  (`self.Translate` (`self.Speed`) (`self.GetActorForwardVector`)))

(fn `Translate`
  (params (speed :type "Float (double-precision)") (direction :type "Vector Structure") (IsSweep :type Boolean))
  (`self.K2_SetActorLocation` (+ (* speed (`GameplayStatics.GetWorldDeltaSeconds`) (`KismetMathLibrary.Normal` direction)) (`self.K2_GetActorLocation`)) IsSweep))

(fn `UserConstructionScript`)