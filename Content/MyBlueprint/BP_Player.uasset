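; BP_Player is a player-controlled actor that moves along its right and up axes and fires bullets.
; Each Tick, GetDirection combines horizontal and vertical values into a normalized vector, which Translate scales by Speed and delta time to set location without sweep.
; The FireBullet press spawns BP_Bullet at the Arrow component's world transform.
; Disconnected rotation and movement experiments remain, and GetDirectionVelocity is unused.
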(event `InputAction|FireBullet`
  (params (Key :type "Key Structure"))
  (:`Pressed`
    (`|SpawnActorFromClass` "/Game/MyBlueprint/BP_Bullet.BP_Bullet_C" (`SceneComponent.K2_GetComponentToWorld` (`self.Arrow`)) "Undefined" "MultiplyWithRoot" null null)))

(event `self.ReceiveBeginPlay`)

(event `self.ReceiveTick`
  (params (DeltaSeconds :type "Float (single-precision)"))
  (`self.Translate` (`self.speed`) (`self.GetDirection`)))

(fn `GetDirection`
  (returns (ReturnValue :type "Vector Structure"))
  (return (`KismetMathLibrary.Normal` (+ (* (`self.GetInputAxisValue`) (`self.GetActorRightVector`)) (* (`self.GetInputAxisValue`) (`self.GetActorUpVector`))))))

(fn `GetDirectionVelocity`
  (returns (ReturnValue :type "Vector Structure"))
  (return (`KismetMathLibrary.MakeVector` 0.0 (`self.GetInputAxisValue`) (`self.GetInputAxisValue`))))

(fn `Translate`
  (params (speed :type "Float (double-precision)") (direction :type "Vector Structure") (IsSweep :type Boolean))
  (`self.K2_SetActorLocation` (+ (* speed (`GameplayStatics.GetWorldDeltaSeconds`) (`KismetMathLibrary.Normal` direction)) (`self.K2_GetActorLocation`)) IsSweep))

(fn `UserConstructionScript`)