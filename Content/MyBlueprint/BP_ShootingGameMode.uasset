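; Game mode for a shooting game that tracks the current score and a persistent high-score record.
; On BeginPlay it shows the WBP_Score widget, hides the cursor, switches to game-only input and loads the record from a BP_SaveGame slot, defaulting to zero.
; AddScore accumulates points and, whenever the score beats the record, updates it and immediately saves it through a newly created save object.
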(event `self.ReceiveBeginPlay`
  (bind _returnvalue (`GameplayStatics.GetPlayerController` 0))
  (bind _returnvalue_2 (`|CreateWidget` "/Game/MyBlueprint/WBP_Score.WBP_Score_C"))
  (`UserWidget.AddToViewport` _returnvalue_2 0)
  (set `PlayerController.bShowMouseCursor` false _returnvalue)
  (`WidgetBlueprintLibrary.SetInputMode_GameOnly` _returnvalue)
  (`self.LoadRecord`))

(fn `AddScore`
  (params (Value :type Integer))
  (bind _output_get (set `self.Score` (+ Value (`self.Score`))))
  (if (> _output_get (`self.NewRecord`))
    (set `self.NewRecord` (`self.Score`))
    (`self.SaveRecord`)))

(fn `LoadRecord`
  (bind _returnvalue (`GameplayStatics.DoesSaveGameExist` (`self.SlotName`)))
  (if _returnvalue
    (bind _returnvalue_2 (`GameplayStatics.LoadGameFromSlot` (`self.SlotName`)))
    (bind _asbp_save_game (cast `/Game/MyBlueprint/BP_SaveGame` _returnvalue_2)
      (:`then`
        (set `self.NewRecord` (`/Game/MyBlueprint/BP_SaveGame.SaveNewRecord` _asbp_save_game)))
      (:`CastFailed`
        (set `self.NewRecord` 0 :!label _label)))
    (else
      (goto _label))))

(fn `SaveRecord`
  (`|ExecutionSequence`
    (:`then_0`
      (bind _returnvalue (`GameplayStatics.CreateSaveGameObject` "/Game/MyBlueprint/BP_SaveGame.BP_SaveGame_C"))
      (set `self.SaveGameInstance` _returnvalue))
    (:`then_1`
      (set `/Game/MyBlueprint/BP_SaveGame.SaveNewRecord` (`self.NewRecord`) (`self.SaveGameInstance`)))
    (:`then_2`
      (`GameplayStatics.SaveGameToSlot` (`self.SaveGameInstance`) (`self.SlotName`)))))

(fn `UserConstructionScript`)